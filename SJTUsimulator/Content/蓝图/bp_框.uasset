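; Tetris-style playfield frame that registers itself with the game mode on BeginPlay.
; Its construction script builds bottom and side walls from static meshes sized by grid counts and spacing, plus center and grid-snapped spawn markers.
; 销毁检测 line-traces each row, destroys hit 形状 components in full rows and returns those row indices.
; 对齐 snaps every actor in the level to a 100-unit grid.
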(event `self.ReceiveBeginPlay`
  (set `/Game/蓝图/俄罗斯方块游戏模式.框` self (`/Game/蓝图/自定义函数库.get my game mode`)))

(fn `get location by 行序号`
  (params (NewParam :type Integer))
  (returns (ReturnValue :type "Vector Structure"))
  (return (+ (`self.K2_GetActorLocation`) (`KismetMathLibrary.MakeVector` 0.0 0.0 (* NewParam 100.0)))))

(fn `get 中心location`
  (returns (ReturnValue :type "Vector Structure"))
  (return (`SceneComponent.K2_GetComponentLocation` (`self.中心点`))))

(fn `get 出生 位置`
  (returns (`return location` :type "Vector Structure"))
  (return (`SceneComponent.K2_GetComponentLocation` (`self.出生点`))))

(fn `get 框的高宽`
  (returns (`宽度` :type "Float (double-precision)") (`高度` :type "Float (double-precision)"))
  (return (* (+ (`self.宽格数`) 1) (`self.间隔x`)) (* (+ (`self.高格数`) 1) (`self.间隔y`))))

(fn `UserConstructionScript`
  (bind (`_宽度` `_高度`) (`self.get 框的高宽`))
  (bind (_returnvalue_x _returnvalue_y _returnvalue_z) (`KismetMathLibrary.BreakVector` (`/Game/蓝图/自定义函数库.vector取整` (`self.出生点偏移`) 100.0)))
  (for _index (range (+ (+ (`self.宽格数`) 1) 1))
    (`AddComponent|NODE_AddStaticMeshComponent-0` :`RelativeTransform` (`KismetMathLibrary.MakeTransform` (`KismetMathLibrary.MakeVector` 0.0 (* _index (`self.间隔x`))))))
  (for _index_2 (range 1 (+ (`self.高格数`) 1))
    (bind _returnvalue (* _index_2 (`self.间隔y`)))
    (`AddComponent|NODE_AddStaticMeshComponent-1` :`RelativeTransform` (`KismetMathLibrary.MakeTransform` (`KismetMathLibrary.MakeVector` 0.0 0.0 _returnvalue))) ; 奇数
    (`AddComponent|NODE_AddStaticMeshComponent-2` :`RelativeTransform` (`KismetMathLibrary.MakeTransform` (`KismetMathLibrary.MakeVector` 0.0 (* (+ (`self.宽格数`) 1) (`self.间隔x`)) _returnvalue))) ; 奇数
  )
  (bind _returnvalue_2 (`AddComponent|NODE_AddArrowComponent-0` :`RelativeTransform` (`KismetMathLibrary.MakeTransform` (`KismetMathLibrary.MakeVector` 0.0 (/ `_宽度` 2.0) (/ `_高度` 2.0)) (struct))))
  (set `self.中心点` _returnvalue_2)
  (set `self.出生点偏移` (`KismetMathLibrary.MakeVector` 0.0 _returnvalue_y _returnvalue_z))
  (bind _returnvalue_3 (`AddComponent|NODE_AddBillboardComponent-0` :`RelativeTransform` (`KismetMathLibrary.MakeTransform` (`self.出生点偏移`))))
  (set `self.出生点` _returnvalue_3))

(fn `对齐`
  (bind _outactors (`GameplayStatics.GetAllActorsOfClass` "/Script/Engine.Actor"))
  (for _array_element _outactors
    (`self.K2_SetActorLocation` _array_element (`/Game/蓝图/自定义函数库.vector取整` (`self.K2_GetActorLocation` _array_element) 100.0) false false)))

(fn `检测目标行`
  (params (`目标行` :type Integer))
  (returns (OutHits :type "Array of HitResult Structure") (ReturnValue :type Boolean))
  (bind _returnvalue (`self.get location by 行序号` `目标行`))
  (bind (_outhits _returnvalue_2) (`KismetSystemLibrary.LineTraceMultiForObjects` _returnvalue (+ _returnvalue (* (`self.GetActorRightVector`) 10000.0)) (`|MakeArray` "ObjectTypeQuery2" :!type "EObjectTypeQuery Enum")))
  (return _outhits _returnvalue_2))

(fn `销毁检测`
  (returns (`销毁行` :type "Array of Integer"))
  (locals (`销毁行数` :type "Array of Integer"))
  (for _index (range 1 (+ (`self.高格数`) 1))
    (bind _outhits (`self.检测目标行` _index))
    (if (>= (`KismetArrayLibrary.Array_Length` _outhits) (`self.宽格数`))
      (`KismetArrayLibrary.Array_Add` (`local.销毁行数`) _index)
      (for _array_element _outhits
        (bind (_bblockinghit _binitialoverlap _time _distance _location _impactpoint _normal _impactnormal _physmat _hitactor _hitcomponent) (`GameplayStatics.BreakHitResult` _array_element))
        (bind `_as形状` (cast `/Game/蓝图/形状/形状` _hitactor))
        (`/Game/蓝图/形状/形状.销毁` `_as形状` _hitcomponent))))
  (return (`local.销毁行数`)))
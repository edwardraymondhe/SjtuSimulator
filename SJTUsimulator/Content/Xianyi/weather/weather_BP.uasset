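; Weather controller that toggles the level between clear skies and dark, rainy weather.
; On Tick it watches the Sidescroller game mode's Timesec for two trigger values, then makes a delayed coin-flip roll to switch state.
; A FlipFlop plays or reverses a timeline that blends sky material colors, cloud opacity and light color.
; Rain particles activate after a delay when darkening and stop before the sky clears.
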(event `self.ReceiveTick`
  (params (DeltaSeconds :type "Float (single-precision)"))
  (bind _sky_material (`/Engine/EngineSky/BP_Sky_Sphere.Sky material` (`self.sky_Ref`)))
  (bind _particlesystemcomponent (`Emitter.ParticleSystemComponent` (`self.rain_Ref`)))
  (bind _assidescroller (cast `/Game/timer/Sidescroller` (`GameplayStatics.GetGameMode`)))
  (bind _timesec (`/Game/timer/Sidescroller.Timesec` _assidescroller))
  (if (or (== _timesec 7) (== _timesec 19))
    (`KismetSystemLibrary.Delay` 1.0)
    (if (== (`KismetMathLibrary.RandomInteger` 2) 1)
      (if (`KismetSystemLibrary.IsValid` (`self.sky_Ref`))
        (`/Engine/EditorBlueprintResources/StandardMacros.FlipFlop`
          (:`A`
            (`|ExecutionSequence`
              (:`then_0`
                (bind (_direction _weather_chag) (`Timeline|weather change` :!label _label)
                  (:`Update`
                    (`MaterialInstanceDynamic.SetVectorParameterValue` _sky_material "Zenith Color" (`KismetMathLibrary.LinearColorLerp` (struct :`R` 0.034046 :`G` 0.109247 :`B` 0.295 :`A` 1.0) (struct :`R` 0.1 :`G` 0.1 :`B` 0.1 :`A` 1.0) _weather_chag))
                    (`MaterialInstanceDynamic.SetVectorParameterValue` _sky_material "Horizon Color" (`KismetMathLibrary.LinearColorLerp` (struct :`R` 1.979559 :`G` 2.586644 :`B` 3.0 :`A` 1.0) (struct :`R` 0.025 :`G` 0.025 :`B` 0.025 :`A` 1.0) _weather_chag))
                    (`MaterialInstanceDynamic.SetVectorParameterValue` _sky_material "Cloud Color" (`KismetMathLibrary.LinearColorLerp` (struct :`R` 0.855778 :`G` 0.91902 :`B` 1.0 :`A` 1.0) (struct :`R` 0.020833 :`G` 0.020833 :`B` 0.020833 :`A` 1.0) _weather_chag))
                    (`MaterialInstanceDynamic.SetScalarParameterValue` _sky_material "Cloud Opacity" (`KismetMathLibrary.Lerp` 1.2 5.0 _weather_chag))
                    (`LightComponent.SetLightColor` (`Light.LightComponent` (`self.light_Ref`)) (`KismetMathLibrary.LinearColorLerp` (struct :`R` 0.855778 :`G` 0.91902 :`B` 1.0 :`A` 1.0) (struct :`A` 1.0) _weather_chag) true))))
              (:`then_1`
                (`KismetSystemLibrary.Delay` 5.0)
                (`ActorComponent.Activate` _particlesystemcomponent false))))
          (:`B`
            (`ActorComponent.Deactivate` _particlesystemcomponent)
            (`KismetSystemLibrary.Delay` 3.0)
            (goto _label :!via `Reverse`)))))))

(fn `UserConstructionScript`)
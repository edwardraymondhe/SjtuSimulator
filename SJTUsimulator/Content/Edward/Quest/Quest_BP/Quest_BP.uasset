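; Quest actor that completes its matching active quest on the player character once triggered and all required flags are found.
; Tick checks the flags, completes the active quest referencing this actor, records its display-name-derived QuestName as finished and notifies NPCs sharing that quest.
; Optionally, it adds its non-boss NPC to the player's list, starting every listed NPC's next conversation when the list reaches three.
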(event `self.ReceiveBeginPlay`
  (bind _asthird_person_character_quest (cast `/Game/Edward/ThirdPersonCharacterQuest` (`GameplayStatics.GetPlayerCharacter` 0)))
  (set `self.PlayerRef` _asthird_person_character_quest))

(event `self.ReceiveTick`
  (params (DeltaSeconds :type "Float (single-precision)"))
  (bind _requiredflags (`self.RequiredFlags`))
  (bind _npcs (`/Game/Edward/ThirdPersonCharacterQuest.NPCs` (`self.PlayerRef`)))
  (bind _returnvalue (`KismetArrayLibrary.Array_Length` _npcs))
  (if (`self.TriggerFlag`)
    (set `self.CanTriggerFlag` true)
    (if (> (`KismetArrayLibrary.Array_Length` _requiredflags) 0)
      (for _array_element _requiredflags
        (bind _found (`/Game/Edward/ThirdPersonCharacterQuest.FindRequiredFlag` (`self.PlayerRef`) _array_element))
        (if (not (== _found true))
          (set `self.CanTriggerFlag` false))))
    (if (`self.CanTriggerFlag`)
      (for _array_element_2 (`/Game/Edward/ThirdPersonCharacterQuest.ActiveQuests` (`self.PlayerRef`))
        (bind (_questinfo_questname _questinfo_questdescription _questinfo_actorreference) (break `/Game/Edward/Quest/QuestInfo` (`/Game/Edward/Quest/BP_Quest.QuestInfo` _array_element_2)))
        (if (== self _questinfo_actorreference)
          (`/Game/Edward/ThirdPersonCharacterQuest.QuestComplete` (`self.PlayerRef`) _array_element_2)
          (bind _outactors (`GameplayStatics.GetAllActorsOfClass` "/Game/Edward/NPC.NPC_C"))
          (for _array_element_3 _outactors
            (bind _questref_questname (break `/Game/Edward/Quest/QuestInfo` (`/Game/Edward/NPC.QuestRef` _array_element_3)))
            (if (`KismetTextLibrary.EqualEqual_TextText` _questinfo_questname _questref_questname)
              (`KismetArrayLibrary.Array_AddUnique` (`/Game/Edward/ThirdPersonCharacterQuest.FinishedFlags` (`self.PlayerRef`)) (`self.QuestName`))
              (`/Game/Edward/NPC.EventQuestComplete` _array_element_3)
              (if (`/Game/Edward/NPC.IsBoss` (`self.NpcRef`))
                _
                (elif (`self.IfAddNpc`)
                  (if (<= _returnvalue 2)
                    (`KismetArrayLibrary.Array_AddUnique` _npcs (`self.NpcRef`))
                    (if (== _returnvalue 3)
                      (for _array_element_4 _npcs
                        (`/Game/Edward/NPC.StartNextConv` _array_element_4)))))))))))))

(fn `UserConstructionScript`
  (set `self.QuestName` (`KismetSystemLibrary.GetDisplayName` self)))
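; CollectItem_BP is an item-collection quest that advances the professor NPC's conversation once the player holds every required item.
; Each Tick, it checks RequiredItems against the player's inventory by name through FindItemInPlayer.
; When all are found or the list is empty, it sets TriggerFlag, shows the professor's exclamation mark and calls StartNextConv.
; No guard prevents this repeating on later ticks while the condition holds.
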(event `self.ReceiveTick`
  (params (DeltaSeconds :type "Float (single-precision)"))
  (bind _requireditems (`self.RequiredItems`))
  (bind _professorref (`self.ProfessorRef`))
  (`parent.ReceiveTick` DeltaSeconds)
  (bind _output_get (set `self.AllFindFlag` true))
  (if (> (`KismetArrayLibrary.Array_Length` _requireditems) 0)
    (for _array_element _requireditems
      (bind _found (`self.FindItemInPlayer` _array_element))
      (if (not _found)
        (set `self.AllFindFlag` false)))
    (if _output_get
      (set `self.TriggerFlag` true :!label _label)
      (if true
        (`SceneComponent.SetHiddenInGame` (`/Game/Edward/NPC.Exclamationmark` _professorref) false false)
        (`/Game/Edward/NPC.StartNextConv` _professorref)))
    (else
      (goto _label))))

(fn `FindItemInPlayer`
  (params (FindItem :type String))
  (returns (Found :type Boolean))
  (for _array_element (`/Game/InventorySystem/InventoryComponent.ItemList` (`/Game/Edward/ThirdPersonCharacterQuest.InventoryComponent` (`self.PlayerRef`)))
    (if (== FindItem (`KismetStringLibrary.Conv_NameToString` (`.ItemName_5_EB72B28B48E610342F61A9AEFE83B793` (break `/Game/InventorySystem/S_Item` _array_element))))
      (return true)))
  (return false))

(fn `UserConstructionScript`
  (`parent.UserConstructionScript`))
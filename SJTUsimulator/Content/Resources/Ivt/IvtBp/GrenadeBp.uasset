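; Grenade actor that shows explosion effects and plays a sound when it hits something, then destroys itself.
; The construction script hides the fire and explosion components until impact.
; The Hit event reveals both, waits briefly, hides the fire, activates the explosion, plays the sound at the actor's location and destroys the actor immediately.
; The graph applies no damage or radial force.
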(event `self.ReceiveHit`
  (params (MyComp :type "PrimitiveComponent Object Reference") (Other :type "Actor Object Reference") (OtherComp :type "PrimitiveComponent Object Reference") (bSelfMoved :type Boolean) (HitLocation :type "Vector Structure") (HitNormal :type "Vector Structure") (NormalImpulse :type "Vector Structure") (Hit :type "HitResult Structure (by ref)"))
  (bind _p_explosion (`self.P_Explosion`))
  (`SceneComponent.SetVisibility` (`self.P_Fire`) true false)
  (`SceneComponent.SetVisibility` _p_explosion true false)
  (`KismetSystemLibrary.Delay` 0.1)
  (`SceneComponent.SetVisibility` (`self.P_Fire`) false false)
  (`ActorComponent.Activate` _p_explosion false)
  (`GameplayStatics.PlaySoundAtLocation` "/Game/StarterContent/Audio/Explosion01.Explosion01" (`self.K2_GetActorLocation`) (struct) 1.0 1.0 0.0 null null null)
  (`self.K2_DestroyActor`))

(fn `UserConstructionScript`
  (`SceneComponent.SetVisibility` (`self.P_Explosion`) false false)
  (`SceneComponent.SetVisibility` (`self.P_Fire`) false false))
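; Pickup item Blueprint for the inventory system, configured as apple, banana or grenade with its own mesh, scale and health/energy/mood bonuses set in the Construction Script.
; A sphere overlap shows a pickup text widget and flags the SWAT player in range.
; The player's bound pickup event adds the item to the bag and refreshes the inventory menu.
; Picked-up items are hidden rather than destroyed, with a function to restore them.
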(event `self.ReceiveBeginPlay`
  (bind (_item_item _item_itemimg _item_itemtext) (break `/Game/Resources/Ivt/IvtBp/IvtStruct` (`self.Item`)))
  ;[1 1 1] Create Widget : Text, PickupActor; Ref Character
  (bind _returnvalue (`|CreateWidget` "/Game/UMG/PickupText.PickupText_C")) ; Create UMNG
  (bind _output_get (set `self.pkTextUiWidget` _returnvalue))
  (set `/Game/UMG/PickupText.pkTextCont` _item_itemtext _output_get)
  (set `/Game/UMG/PickupText.pkActor` self _output_get)
  (bind _asswat_player_character (cast `/Game/Player/PlayerBP/SwatPlayerCharacter` (`GameplayStatics.GetPlayerCharacter` 0)))
  (set `self.swatInst` _asswat_player_character)
  (add `/Game/Player/PlayerBP/SwatPlayerCharacter.SwatPickup` (`self.swatInst`) (delegate `ItemPickup`)))

(event `ItemPickup`
  ;[1 1 1] Create Widget : Text, PickupActor; Ref Character
  ;[1 1 1] Add Item
  (if (and (`self.GetActorEnableCollision`) (`self.isSwatInRange`))
    (`KismetArrayLibrary.Array_Add` (`/Game/Player/PlayerBP/SwatPlayerCharacter.bagIvt` (`self.swatInst`)) (`self.Item`))
    (`self.PkItemRemoveFromView`)
    (set `self.isSwatInRange` false)
    (`/Game/UMG/UmgHUD.RefreshIvtMenu` (`/Game/Player/PlayerBP/SwatPlayerCharacter.myGameHud` (`self.swatInst`)))))

(event `self.Sphere.OnComponentBeginOverlap`
  (params (OverlappedComponent :type "PrimitiveComponent Object Reference") (OtherActor :type "Actor Object Reference") (OtherComp :type "PrimitiveComponent Object Reference") (OtherBodyIndex :type Integer) (bFromSweep :type Boolean) (SweepResult :type "HitResult Structure (by ref)"))
  ;[1 1 1] Overlap
  (cast `/Game/Player/PlayerBP/SwatPlayerCharacter` OtherActor)
  (if (not (`Widget.IsInViewport` (`self.pkTextUiWidget`)))
    (`UserWidget.AddToViewport` (`self.pkTextUiWidget`) 0)
    (set `self.isSwatInRange` true)))

(event `self.Sphere.OnComponentEndOverlap`
  (params (OverlappedComponent :type "PrimitiveComponent Object Reference") (OtherActor :type "Actor Object Reference") (OtherComp :type "PrimitiveComponent Object Reference") (OtherBodyIndex :type Integer))
  ;[1 1 1] Overlap
  (cast `/Game/Player/PlayerBP/SwatPlayerCharacter` OtherActor)
  (if (`Widget.IsInViewport` (`self.pkTextUiWidget`))
    (`Widget.RemoveFromParent` (`self.pkTextUiWidget`))
    (set `self.isSwatInRange` false)))

(fn `PkItemAddView`
  (`PrimitiveComponent.SetCollisionEnabled` (`self.Sphere`) "QueryOnly")
  (`SceneComponent.SetVisibility` (`self.StaticMesh`) true false)
  (if (not (`Widget.IsInViewport` (`self.pkTextUiWidget`)))
    (`UserWidget.AddToViewport` (`self.pkTextUiWidget`) 0)))

(fn `PkItemRemoveFromView`
  (`PrimitiveComponent.SetCollisionEnabled` (`self.Sphere`) "NoCollision")
  (`SceneComponent.SetVisibility` (`self.StaticMesh`) false false)
  (`Widget.RemoveFromParent` (`self.pkTextUiWidget`)) ; Remove Text
)

(fn `setAddHem`
  (params (parHealth :type "Float (double-precision)") (ParEnergy :type "Float (double-precision)") (parMood :type "Float (double-precision)"))
  (set `self.addHealth` parHealth)
  (set `self.AddEnergy` ParEnergy)
  (set `self.addMood` parMood))

(fn `UserConstructionScript`
  (bind _ivtchoose (`self.IvtChoose`))
  (bind (_mesh _image _name) (break `/Game/Resources/Ivt/IvtBp/IvtRaw` (`|GetArrayItem` (`self.IvtList`) (`KismetMathLibrary.Conv_ByteToInt` _ivtchoose))))
  ;[1 1 1] Set ItemInfo Values
  (`StaticMeshComponent.SetStaticMesh` (`self.StaticMesh`) _mesh)
  (set `self.Item` (make `/Game/Resources/Ivt/IvtBp/IvtStruct` self _image _name))
  ;[1 1 1] Set Scale and HEM
  (switch `/Game/Resources/Ivt/IvtBp/IvtEnum` _ivtchoose
    (:`NewEnumerator0`
      (`SceneComponent.SetWorldScale3D` (`self.StaticMesh`) (0.3 0.3 0.3))
      (`self.setAddHem` 0.1 0.1 0.02))
    (:`NewEnumerator1`
      (`SceneComponent.SetWorldScale3D` (`self.StaticMesh`) (1.5 1.5 1.5))
      (`self.setAddHem` 0.1 0.15 0.02))
    (:`NewEnumerator2`
      (`SceneComponent.SetWorldScale3D` (`self.StaticMesh`) (3.0 3.0 3.0))
      (`self.setAddHem` 0.0 0.0 0.05))))